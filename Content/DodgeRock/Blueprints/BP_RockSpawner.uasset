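; Spawner actor for DodgeRock that creates BP_Rock actors at random positions within a box, with damage scaled by game difficulty.
; On BeginPlay it reads the difficulty from BP_DodgeRockGameInstance and picks the rock base damage for Easy, Medium or Hard.
; SpawnRockInVolume takes random X and Y inside the Box bounds, keeps the spawner's own height, and passes that damage to each rock.
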(event Custom|SpawnRockInVolume
  (bind _box (Variables|Default|GetBox))
  (bind _returnvalue (Transformation|GetWorldLocation _box))
  (bind _returnvalue_2 (Components|Box|GetScaledBoxExtent _box))
  (bind _returnvalue_3 (Math|Random|RandomPointinBoundingBox _returnvalue _returnvalue_2))
  (bind (_x _y) (Class|KismetMathLibrary|BreakVector3f _returnvalue_3))
  (Game|SpawnActorfromClass "/Game/DodgeRock/Blueprints/BP_Rock.BP_Rock_C" (Math|Transform|MakeTransform (Math|Vector|MakeVector _x _y (.Z (Class|KismetMathLibrary|BreakVector3f (Transformation|GetActorLocation))))) "AdjustIfPossibleButAlwaysSpawn" 0 (Variables|Default|GetRockBaseDamage) 0))

(event EventBeginPlay
  (bind _asbp_dodge_rock_game_instance (Utilities|Casting|CastToBP_DodgeRockGameInstance (Game|GetGameInstance)))
  (Variables|Default|SetRockBaseDamage (Utilities|Select :Index (Default|GetGameDifficulty _asbp_dodge_rock_game_instance) :NewEnumerator0 25.0 :NewEnumerator1 5e+01 :NewEnumerator2 1e+02)))

(fn ConstructionScript)